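; BP_Button is a numbered pedestal button that spawns an AITurtle when used.
; UseButton fires once through a DoOnce, playing a sound and a timeline that offsets the button's Z, then spawns the turtle with start and end points and the pedestal number.
; Box overlaps by ThirdPersonCharacter toggle a text hint, while the construction script labels the pedestal with NumberPedestal + 1 and caches the button's location.
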(event OnComponentBeginOverlap(Box)
  (params (OverlappedComponent :type Primitive%20Component%20Object%20Reference) (OtherActor :type Actor%20Object%20Reference) (OtherComp :type Primitive%20Component%20Object%20Reference) (OtherBodyIndex :type Integer) (bFromSweep :type Boolean) (SweepResult :type Hit%20Result%20Structure%20%28by%20ref%29))
  ;[1 1 1] Показывает подсказку какую кнопку нажимать
  (if (== (Utilities|GetClass OtherActor) "/Game/Project/Blueprints/ThirdPersonCharacter.ThirdPersonCharacter_C")
    (Rendering|SetVisibility (Variables|Default|GetTextRender1) true false)))

(event OnComponentEndOverlap(Box)
  (params (OverlappedComponent :type Primitive%20Component%20Object%20Reference) (OtherActor :type Actor%20Object%20Reference) (OtherComp :type Primitive%20Component%20Object%20Reference) (OtherBodyIndex :type Integer))
  ;[1 1 1] Показывает подсказку какую кнопку нажимать
  (if (== (Utilities|GetClass OtherActor) "/Game/Project/Blueprints/ThirdPersonCharacter.ThirdPersonCharacter_C")
    (Rendering|SetVisibility (Variables|Default|GetTextRender1) false false)))

(event EventUseButton
  (bind _returnvalue (Transformation|GetActorLocation))
  (bind _buttonlocation (Variables|Default|GetButtonLocation))
  (bind _returnvalue_2 (+ _returnvalue "50.000000,0.000000,-330.000000"))
  (Utilities|FlowControl|DoOnce false
    (:Completed
      ;[1 1 1] Нажатие кнопки
      (Audio|SpawnSoundatLocation "/Game/Project/Sound/Button_Cue.Button_Cue" (Transformation|GetActorLocation) "0, 0, 0" 1.0 1.0 0.0 0 0)
      (bind _newtrack_0 (Timeline|Timeline_0 Play)
        (:Update
          (Transformation|SetRelativeLocation (Variables|Default|GetButton) (Math|Vector|MakeVector (.x _buttonlocation) (.y _buttonlocation) (+ (.z _buttonlocation) _newtrack_0)) false false))
        (:Finished
          ;[1 1 1] Спавн черепахи
          (Game|SpawnActorfromClass "/Game/Project/AI/AITurtle.AITurtle_C" (Math|Transform|MakeTransform _returnvalue_2 "0.000000,90.000000, 0" "1,1,1") "Undefined" 0 _returnvalue_2 (+ _returnvalue "50.000000,3500.000000,-330.000000") (Variables|Default|GetNumber%20Pedestal) 0))))))

(fn ConstructionScript
  (Rendering|Components|TextRender|SetText (Variables|Default|GetTextRender) (Utilities|Text|ToText(Integer) (+ (Variables|Default|GetNumber%20Pedestal) 1)))
  (Variables|Default|SetButtonLocation (Variables|/Script/Engine.SceneComponent|GetRelativeLocation (Variables|Default|GetButton))))